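; BP_FollowingCube is a cube that turns toward the first-person player, then requests an equipment loot drop and destroys itself when hit.
; BeginPlay caches the player, and Tick sets the cube's relative yaw from an unsigned dot-product angle to the player, printing it for debugging.
; A right-vector angle is used only when the forward angle is zero.
; Pawn sensing is empty and the AIMoveTo chase is unwired, so it never moves.
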(event OnSeePawn(PawnSensing)
  (params (Pawn :type Pawn%20Object%20Reference)))

(event Custom|TakenHit
  (Class|BPISpawnLoot|SpawnLootRequest(Message) (Game|GetGameMode) (Transformation|GetActorLocation) "NewEnumerator3" "(TagName=\"Equipment\")")
  (Actor|DestroyActor))

(event EventTick
  (params (DeltaSeconds :type Float%20%28single-precision%29))
  (bind _returnvalue (Transformation|GetActorLocation))
  (bind _returnvalue_2 (Transformation|GetActorForwardVector))
  (bind _playerref (Variables|Default|GetPlayerRef))
  (bind _returnvalue_3 (Transformation|GetActorLocation _playerref))
  (bind _returnvalue_4 (Math|Vector|Normalize _returnvalue_2))
  (bind _returnvalue_5 (- _returnvalue_3 _returnvalue))
  (bind _returnvalue_6 (Math|Vector|Normalize _returnvalue_5))
  (bind _returnvalue_7 (Math|Vector|DotProduct _returnvalue_6 _returnvalue_4))
  (bind _returnvalue_8 (Class|KismetMathLibrary|DegAcos _returnvalue_7))
  (Development|PrintString (Utilities|String|ToString(Float) _returnvalue_8))
  (if (> _returnvalue_8 0.0)
    (Transformation|SetRelativeRotation (Variables|Default|GetCube) (Math|Rotator|MakeRotator 0.0 0.0 _returnvalue_8) false false)
    (else
      (Transformation|SetRelativeRotation (Variables|Default|GetCube) (Math|Rotator|MakeRotator 0.0 0.0 (Class|KismetMathLibrary|DegAcos (Math|Vector|DotProduct (Math|Vector|Normalize (- (Transformation|GetActorLocation (Variables|Default|GetPlayerRef)) (Transformation|GetActorLocation))) (Math|Vector|Normalize (Transformation|GetActorRightVector))))) false false))))

(event EventBeginPlay
  (bind _outactors (Actor|GetAllActorsOfClass "/Game/FirstPerson/Blueprints/BP_FirstPersonCharacter.BP_FirstPersonCharacter_C"))
  (Variables|Default|SetPlayerRef (Utilities|Array|Get(acopy) _outactors)))

(fn ConstructionScript)