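; BP_FollowCam is a follow-camera actor that tracks the first-person character.
; Every Tick it looks up BP_FirstPersonCharacter with GetAllActorsOfClass and takes the first result, without caching it.
; It moves its root to that character's location plus the TargetCameraPos offset, without sweeping.
; Root rotation is built by MakeRotationFromAxes from only the character rotation's X component, with Right and Up zeroed.
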(event EventBeginPlay)

(event Collision|EventActorBeginOverlap
  (params (OtherActor :type Actor%20Object%20Reference)))

(event EventTick
  (params (DeltaSeconds :type Float%20%28single-precision%29))
  (bind _defaultsceneroot (Variables|Default|GetDefaultSceneRoot))
  (bind _outactors (Actor|GetAllActorsOfClass "/Game/FirstPerson/Blueprints/BP_FirstPersonCharacter.BP_FirstPersonCharacter_C"))
  (Transformation|SetWorldLocation _defaultsceneroot (+ (Transformation|GetActorLocation (Utilities|Array|Get(acopy) _outactors)) (Variables|Default|GetTargetCameraPos)) false false)
  (Transformation|SetWorldRotation _defaultsceneroot (Math|Rotator|MakeRotationfromAxes (.X (Math|Rotator|BreakRotIntoAxes (Transformation|GetActorRotation (Utilities|Array|Get(acopy) _outactors)))) "0, 0, 0" "0, 0, 0") false false))

(fn ConstructionScript)