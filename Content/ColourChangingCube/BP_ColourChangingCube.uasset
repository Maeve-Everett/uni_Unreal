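; BP_ColourChangingCube is a cube actor whose material colour can be set and randomised at runtime.
; The construction script creates a dynamic material instance on the cube's first material slot, stores it, and applies the Colour variable to its "Colour" parameter.
; A RandomiseColour event picks random RGB values with zero alpha and pushes them to that stored material instance.
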(event Custom|RandomiseColour
  (bind _output_get (Variables|Default|SetColour (Utilities|Struct|MakeLinearColor (Math|Random|RandomFloat) (Math|Random|RandomFloat) (Math|Random|RandomFloat) 0.0)))
  (Rendering|Material|SetVectorParameterValue (Variables|Default|GetNewVar_0) "Colour" _output_get :!class /Script/Engine.MaterialInstanceDynamic))

(event EventBeginPlay)

(event Collision|EventActorBeginOverlap
  (params (OtherActor :type Actor%20Object%20Reference)))

(fn ConstructionScript
  (bind _returnvalue (Rendering|Material|CreateDynamicMaterialInstance (Variables|Default|GetCube) 0 0 "None" :!class /Script/Engine.PrimitiveComponent))
  (Variables|Default|SetNewVar_0 _returnvalue)
  (Rendering|Material|SetVectorParameterValue _returnvalue "Colour" (Variables|Default|GetColour) :!class /Script/Engine.MaterialInstanceDynamic))